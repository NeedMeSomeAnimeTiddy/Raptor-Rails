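; Train actor that runs along the BP_TrainSpline rail, puffing smoke from its funnel on a looping timer and carrying enemies.
; Construction script snaps it to the spline and adds a coal carriage plus passenger carriages, alternating two kinds via FlipFlop.
; Tick advances the front by Speed, and UpdateTrain places each carriage at an offset spline distance, wrapping negative distances by spline length.
; BeginPlay attaches three BP_ThirdPersonCharacter enemies to sockets on each passenger carriage.
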(event Custom|Smoke%20Effect
  (bind _mesh (Variables|Default|GetMesh))
  (Niagara|SpawnSystematLocation "/Game/Gun/Niagara/NG_TrainSmoke.NG_TrainSmoke" (Transformation|GetSocketLocation _mesh "Funnel") (Transformation|GetWorldRotation _mesh)))

(event EventBeginPlay
  (Utilities|Time|SetTimerbyEvent (delegate Custom|Smoke%20Effect) 0.125 true)
  (for _array_element (Variables|Components|GetPassengerCarriages)
    (for _index (range 0 2)
      (Utilities|SpawnEnemy (Utilities|Select :Index _index :Option%200 "EnemyTop1" :Option%201 "EnemyTop2" :Option%202 "EnemyBalcony") _array_element))))

(event EventTick
  (params (DeltaSeconds :type Float%20%28single-precision%29))
  (bind _rail_spline (Variables|Default|GetRail%20Spline)
    (:then
      (Transformation|SetActorLocationAndRotation (Spline|GetLocationatDistanceAlongSpline _rail_spline (Variables|Default|GetTrainFrontTrackDistance) "World") (Spline|GetRotationatDistanceAlongSpline _rail_spline (Variables|Default|GetTrainFrontTrackDistance) "World"))
      (Variables|Default|SetTrainFrontTrackDistance (+ (Variables|Default|GetTrainFrontTrackDistance) (* (Variables|Default|GetSpeed) (Utilities|Time|GetWorldDeltaSeconds))))
      (CallFunction|UpdateTrain))
    (:else)))

(fn ConstructionScript
  (bind _passengercarriages (Variables|Components|GetPassengerCarriages))
  (bind _trainfronttrackdistance (Variables|Default|GetTrainFrontTrackDistance))
  (bind _returnvalue (Actor|GetActorOfClass "/Game/Gun/Train/BP_TrainSpline.BP_TrainSpline_C"))
  (bind _output_get (Variables|Default|SetRail%20Spline (Variables|/Game/Gun/Train/BP_TrainSpline.BP_TrainSpline_C|GetSpline _returnvalue)))
  (Transformation|SetActorLocationAndRotation (Spline|GetLocationatDistanceAlongSpline _output_get _trainfronttrackdistance "World") (Spline|GetRotationatDistanceAlongSpline _output_get _trainfronttrackdistance "World"))
  (bind _returnvalue_2 (AddComponent|AddSkeletalMeshComponent false (Math|Transform|MakeTransform (Math|Vector|MakeVector (* (Variables|Customization|GetCoalCarriageLength) -1.0) 0.0 0.0) "0.000000,-90.000000,0.000000" "1.000000,1.000000,1.000000")))
  (Variables|Default|SetCoalCarriage _returnvalue_2)
  (for _index (range 1 (Variables|Customization|GetPassengerCarriageCount))
    (Utilities|FlowControl|FlipFlop
      (:A
        (bind _returnvalue_3 (AddComponent|AddSkeletalMeshComponent false (Math|Transform|MakeTransform (Math|Vector|MakeVector (+ (* _index (Variables|Customization|GetPassengerCarriageLength) -1.0) -721.0) 0.0 0.0) "0.000000,-90.000000,0.000000" "1.000000,1.000000,1.000000")))
        (bind _output_get_2 (Variables|Default|SetPassengerCarriage1 _returnvalue_3))
        (Utilities|Array|AddUnique _passengercarriages _output_get_2))
      (:B
        (bind _returnvalue_4 (AddComponent|AddSkeletalMeshComponent false (Math|Transform|MakeTransform (Math|Vector|MakeVector (+ (* _index (Variables|Customization|GetPassengerCarriageLength) -1.0) -721.0) 0.0 0.0) "0.000000,-90.000000,0.000000" "1.000000,1.000000,1.000000")))
        (bind _output_get_3 (Variables|Default|SetPassengerCarriage2 _returnvalue_4))
        (Utilities|Array|AddUnique _passengercarriages _output_get_3))))
  (CallFunction|UpdateTrain))

(fn UpdateTrain
  (bind _trainfronttrackdistance (Variables|Default|GetTrainFrontTrackDistance))
  (bind _coalcarriagelength (Variables|Customization|GetCoalCarriageLength))
  (bind _rail_spline (Variables|Default|GetRail%20Spline))
  (bind _rail_spline_2 (Variables|Default|GetRail%20Spline))
  (bind _returnvalue (* _coalcarriagelength -1.0))
  (bind _returnvalue_2 (+ _returnvalue _trainfronttrackdistance 0.0))
  (if (<= _returnvalue_2 0.0)
    (LocalVariables|SetCoalTrackDistance (+ _returnvalue_2 (Spline|GetSplineLength (Variables|Default|GetRail%20Spline))))
    (else
      (LocalVariables|SetCoalTrackDistance _returnvalue_2)))
  (Transformation|SetWorldLocationAndRotation (Variables|Default|GetCoalCarriage) (Spline|GetLocationatDistanceAlongSpline _rail_spline (LocalVariables|GetCoalTrackDistance) "World") (Math|Rotator|MakeRotator (* (.Pitch (Math|Rotator|BreakRotator (Spline|GetRotationatDistanceAlongSpline _rail_spline (LocalVariables|GetCoalTrackDistance) "World"))) -1.0) (.Roll (Math|Rotator|BreakRotator (Spline|GetRotationatDistanceAlongSpline _rail_spline (LocalVariables|GetCoalTrackDistance) "World"))) (+ (.Yaw (Math|Rotator|BreakRotator (Spline|GetRotationatDistanceAlongSpline _rail_spline (LocalVariables|GetCoalTrackDistance) "World"))) -9e+01)) false false)
  (for (_array_element _array_index) (Variables|Components|GetPassengerCarriages)
    (if (<= (+ (* _array_index (Variables|Customization|GetPassengerCarriageLength) -1.0) (Variables|Default|GetTrainFrontTrackDistance) (- -1.45e+03 (Variables|Customization|GetCoalCarriageLength))) 0.0)
      (LocalVariables|SetCarriageTrackDistance (+ (+ (* _array_index (Variables|Customization|GetPassengerCarriageLength) -1.0) (Variables|Default|GetTrainFrontTrackDistance) (- -1.45e+03 (Variables|Customization|GetCoalCarriageLength))) (Spline|GetSplineLength (Variables|Default|GetRail%20Spline))))
      (else
        (LocalVariables|SetCarriageTrackDistance (+ (* _array_index (Variables|Customization|GetPassengerCarriageLength) -1.0) (Variables|Default|GetTrainFrontTrackDistance) (- -1.45e+03 (Variables|Customization|GetCoalCarriageLength))))))
    (Transformation|SetWorldLocationAndRotation _array_element (Spline|GetLocationatDistanceAlongSpline _rail_spline_2 (LocalVariables|GetCarriageTrackDistance) "World") (Math|Rotator|MakeRotator (* (.Pitch (Math|Rotator|BreakRotator (Spline|GetRotationatDistanceAlongSpline _rail_spline_2 (LocalVariables|GetCarriageTrackDistance) "World"))) -1.0) (.Roll (Math|Rotator|BreakRotator (Spline|GetRotationatDistanceAlongSpline _rail_spline_2 (LocalVariables|GetCarriageTrackDistance) "World"))) (+ (.Yaw (Math|Rotator|BreakRotator (Spline|GetRotationatDistanceAlongSpline _rail_spline_2 (LocalVariables|GetCarriageTrackDistance) "World"))) -9e+01)) false false)
    (for _index (range 1 4)
      _)))