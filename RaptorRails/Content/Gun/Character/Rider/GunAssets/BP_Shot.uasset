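; BP_Shot is a short-lived actor that resolves one delayed hitscan gunshot from BP_Rider.
; On BeginPlay it copies the rider's shot values and uses ShotDistance as a timer delay before tracing, damaging the hit actor and destroying itself.
; LineTrace spawns a bullet-hole decal, a surface-based sound at the muzzle and a deflect effect oriented along the reflected ricochet direction.
; Only stone, metal and default surfaces have sounds and effects assigned.
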(event Custom|Shoot
  (CallFunction|LineTrace)
  (Game|Damage|ApplyDamage (Variables|Default|GetHit%20Actor) (Variables|Default|GetShot%20Damage) 0 0)
  (Actor|DestroyActor))

(event EventBeginPlay
  ;[1 1 1] Referencing
  (bind _returnvalue (Actor|GetActorOfClass "/Game/Gun/Character/Rider/BP_Rider.BP_Rider_C"))
  (bind _output_get (Variables|Default|SetAs%20BP%20Rider _returnvalue))
  (Utilities|FlowControl|Sequence
    (:then_0
      (Variables|Linetracing|SetMuzzle%20Location (Variables|/Game/Gun/Character/Rider/BP_Rider.BP_Rider_C|GetMuzzleLocation _output_get)))
    (:then_1
      (Variables|Linetracing|SetShot%20Location (Variables|/Game/Gun/Character/Rider/BP_Rider.BP_Rider_C|GetShotLocation _output_get)))
    (:then_2
      (Variables|Linetracing|SetShot%20Distance (Variables|/Game/Gun/Character/Rider/BP_Rider.BP_Rider_C|GetShotDistance _output_get)))
    (:then_3
      (Variables|Linetracing|SetAmmo%20Combo (Variables|/Game/Gun/Character/Rider/BP_Rider.BP_Rider_C|GetAmmoCombo _output_get)))
    (:then_4
      (Variables|Linetracing|SetRange (Variables|/Game/Gun/Character/Rider/BP_Rider.BP_Rider_C|GetRange _output_get))
      (Utilities|Time|SetTimerbyEvent (delegate Custom|Shoot) (Variables|Linetracing|GetShot%20Distance)))
    (:then_5
      (Variables|Default|SetShot%20Damage (Variables|/Game/Gun/Character/Rider/BP_Rider.BP_Rider_C|GetShotDamage _output_get)))))

(fn ConstructionScript)

(fn LineTrace
  (bind _outhit (Collision|LineTraceByChannel (Variables|Linetracing|GetMuzzle%20Location) (Variables|Linetracing|GetShot%20Location) "TraceTypeQuery1" false 0 "None"))
  (Utilities|FlowControl|Sequence
    (:then_0
      (LocalVariables|SetHitLocation (.ImpactPoint (Collision|BreakHitResult _outhit))))
    (:then_1
      (LocalVariables|SetHitNormal (.ImpactNormal (Collision|BreakHitResult _outhit))))
    (:then_2
      (Variables|Default|SetHit%20Actor (.HitActor (Collision|BreakHitResult _outhit))))
    (:then_3
      (Variables|Default|SetHit%20Component (.HitComponent (Collision|BreakHitResult _outhit))))
    (:then_4
      (LocalVariables|SetHitSurfaceType (Collision|GetSurfaceType _outhit)))
    (:then_5
      (LocalVariables|SetRicochetLocation (+ (LocalVariables|GetHitLocation) (* (Math|Vector|GetReflectionVector (Math|Vector|GetUnitDirection(Vector) (.TraceStart (Collision|BreakHitResult _outhit)) (.TraceEnd (Collision|BreakHitResult _outhit))) (LocalVariables|GetHitNormal)) (Variables|Linetracing|GetRange))))
      (Class|GameplayStatics|SpawnDecalAttached "/Game/Gun/Materials/BulletHole.BulletHole" "50.000000,50.000000,50.000000" (Variables|Default|GetHit%20Component) "None" (LocalVariables|GetHitLocation) (Math|Conversions|RotationFromXVector (LocalVariables|GetHitNormal)) "KeepRelativeOffset" 1e+01)
      (bind _outhit_2 (Collision|LineTraceByChannel (LocalVariables|GetHitLocation) (LocalVariables|GetRicochetLocation) "TraceTypeQuery1" false 0 "None"))
      (LocalVariables|SetRicochetDirection (Math|Conversions|RotationFromXVector (Math|Vector|GetUnitDirection(Vector) (.TraceStart (Collision|BreakHitResult _outhit_2)) (.TraceEnd (Collision|BreakHitResult _outhit_2)))))
      (Audio|PlaySoundatLocation (Utilities|Select :Index (LocalVariables|GetHitSurfaceType) :SurfaceType_Default (Utilities|Select :Index (Math|Random|RandomIntegerinRange 0 3) :Option%200 "/Game/Gun/SFX/HitEffects/HitStone1.HitStone1" :Option%201 "/Game/Gun/SFX/HitEffects/HitStone2.HitStone2" :Option%202 "/Game/Gun/SFX/HitEffects/HitStone3.HitStone3" :Option%203 "/Game/Gun/SFX/HitEffects/HitStone4.HitStone4") :SurfaceType1 (Utilities|Select :Index (Math|Random|RandomIntegerinRange 0 3) :Option%200 "/Game/Gun/SFX/HitEffects/HitStone1.HitStone1" :Option%201 "/Game/Gun/SFX/HitEffects/HitStone2.HitStone2" :Option%202 "/Game/Gun/SFX/HitEffects/HitStone3.HitStone3" :Option%203 "/Game/Gun/SFX/HitEffects/HitStone4.HitStone4") :SurfaceType2 (Utilities|Select :Index (Math|Random|RandomIntegerinRange 0 3) :Option%200 "/Game/Gun/SFX/HitEffects/HitMetal1.HitMetal1" :Option%201 "/Game/Gun/SFX/HitEffects/HitMetal2.HitMetal2" :Option%202 "/Game/Gun/SFX/HitEffects/HitMetal3.HitMetal3" :Option%203 "/Game/Gun/SFX/HitEffects/HitMetal4.HitMetal4") :SurfaceType3 (Utilities|Select :Index (Math|Random|RandomIntegerinRange 0 3) :Option%200 0 :Option%201 0 :Option%202 0 :Option%203 0) :SurfaceType4 (Utilities|Select :Index (Math|Random|RandomIntegerinRange 0 3) :Option%200 0 :Option%201 0 :Option%202 0 :Option%203 0)) (Variables|Linetracing|GetMuzzle%20Location) "0, 0, 0" 1.0 1.0 0.0 0 0 0 0)
      (Niagara|SpawnSystematLocation (Utilities|Select :Index (LocalVariables|GetHitSurfaceType) :SurfaceType_Default "/Game/Gun/Niagara/NS_StoneDeflect.NS_StoneDeflect" :SurfaceType1 "/Game/Gun/Niagara/NS_StoneDeflect.NS_StoneDeflect" :SurfaceType2 "/Game/Gun/Niagara/NS_MetalDeflect.NS_MetalDeflect" :SurfaceType3 0 :SurfaceType4 0) (LocalVariables|GetHitLocation) (LocalVariables|GetRicochetDirection))
      (return))))