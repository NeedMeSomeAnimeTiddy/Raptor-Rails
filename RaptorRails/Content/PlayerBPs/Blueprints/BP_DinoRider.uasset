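; BP_DinoRider is the player's raptor mount character, with HUD, camera shakes, delayed health regeneration and an assisted-steering "Dynamic Raptor" system.
; Each tick, sphere and line traces drive turning, dodging, enemy kills, ledge braking and height-scaled jumps, adjusting walk speed alongside the controller's RegulateSpeed timer.
; With no obstacle hits, it aligns to the nearest nearby BP_DRSpline.
; Manual movement, jumping or high speed suspends the assist through a short cooldown.
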(event EventTick
  (params (DeltaSeconds :type Float%20%28single-precision%29))
  (Variables|Default|SetDelta%20Seconds DeltaSeconds)
  ;[0 1 0.003875] Submission
  (DynamicRaptor|DynamicRaptor))

(fn ConstructionScript)

(fn HUD
  (bind _returnvalue (UserInterface|CreateWidget "/Game/UI/WB_Reticle.WB_Reticle_C"))
  (Variables|Default|SetReticleREF _returnvalue)
  (bind _returnvalue_2 (UserInterface|CreateWidget "/Game/UI/WB_HUD.WB_HUD_C"))
  (UserInterface|Viewport|AddtoViewport _returnvalue_2 0))

(fn RecoverHealth
  (bind _output_get (Variables|Default|SetHealth (Math|Interpolation|FInterpTo (Variables|Default|GetHealth) 1e+02 (Variables|Default|GetDelta%20Seconds) 1.0))))

(fn DynamicRaptor
  (bind _as_player_controller (Variables|Default|GetAs%20Player%20Controller))
  (bind _as_player_controller_2 (Variables|Default|GetAs%20Player%20Controller))
  (if (Math|Boolean|ORBoolean (Input|EnhancedActionValues|GetIA_MoveReset) (not (Character|CanJump)) (> (Math|Vector|VectorLength (Transformation|GetVelocity)) 1.6e+03) (Utilities|Time|IsTimerActivebyHandle (Variables|DynamicRaptor|GetDRCDTimerHandle)))
    ;[0 0.9605 1] Cooldown Trigger
    (CallFunction|Cooldown)
    (else
      (Utilities|FlowControl|Sequence
        (:then_0
          ;[0.9431 1 0.3781] Enemy Killed by Turning EKT
          ;;[1 0.2946 0.274] Middle Trace
          (bind (_returnvalue _outhit) (DynamicRaptor|SphereTraceDR 6e+01 0.0 0.0 0.0 0.0 0.1 3e+02 "TraceTypeQuery4"))
          ;;[0.4156 1 0.374] Kill Enemy Based on trace hit
          (DynamicRaptor|TracesHittingDR _returnvalue)
          (if _returnvalue
            (bind (_rotating _hitactor) (DynamicRaptor|RotateDR _outhit 3.0 false true true 0.0 3e+01 true 3e+01 true))
            (if (not _rotating)
              (Actor|DestroyActor _hitactor))))
        (:then_1
          ;[0.9431 1 0.3781] Stop Falling Off Ledge SFOL
          ;;[1 0.2946 0.274] Down Trace
          (bind _returnvalue_2 (DynamicRaptor|SphereTraceDR -1e+02 0.0 0.0 0.0 2.5e+02 0.1 15.0 "TraceTypeQuery2"))
          ;;[0.4156 1 0.374] Ledge Stop Trace Hit
          (if _returnvalue_2
            (Class|KismetSystemLibrary|UnPauseTimer _as_player_controller "RegulateSpeed")
            (else
              (Class|KismetSystemLibrary|PauseTimer _as_player_controller "RegulateSpeed")
              (bind _returnvalue_3 (DynamicRaptor|LineTraceDR 2.5e+02 -1e+02 -1.5e+02 0.0 "TraceTypeQuery1"))
              (if (not _returnvalue_3)
                (Utilities|SlowDown 0.0 3e+03 6e+01)))))
        (:then_2
          ;[0.9431 1 0.3781] Avoid Front Obstacles AFO
          ;;[1 0.2946 0.274] Forward Trace
          (bind (_returnvalue_4 _outhit_2) (DynamicRaptor|SphereTraceDR 6e+01 5.0 0.0 0.0 0.0 6e+02 6e+01 "TraceTypeQuery1"))
          ;;[0.4823 1 0.517] Turn Based on Impact Location rotation relative to player rotation
          (DynamicRaptor|TracesHittingDR _returnvalue_4)
          (if _returnvalue_4
            (bind _rotating_2 (DynamicRaptor|RotateDR _outhit_2 1.0 true false false 0.0 0.5 false 3e+01 false))
            (if (not _rotating_2)
              ;;[0.4823 1 0.517] No Trace Hit speed back to normal
              (GameplayTags|RemoveGameplayTag (Variables|/Game/PlayerBPs/Blueprints/BP_PlayerController.BP_PlayerController_C|GetGameplayTags _as_player_controller_2) "(TagName=\"Player.State.Avoiding\")" :!class /Script/GameplayTags.BlueprintGameplayTagLibrary)
              (Class|KismetSystemLibrary|UnPauseTimer _as_player_controller_2 "RegulateSpeed"))))
        (:then_3
          ;[0.9431 1 0.3781] Avoid Falling Obstacles Dodge AFOD
          ;;[1 0.2946 0.274] Up Trace
          (bind (_returnvalue_5 _outhit_3) (DynamicRaptor|SphereTraceDR 2.4e+02 4e+01 0.0 0.0 0.0 8e+02 8e+01 "TraceTypeQuery3"))
          ;;[0.4156 1 0.374] Dodge Trace Hit
          (DynamicRaptor|TracesHittingDR _returnvalue_5)
          (if _returnvalue_5
            (DynamicRaptor|RotateDR _outhit_3 4.0 false false false 0.0 0.0 false 0.0 true)))
        (:then_4
          ;[0.9431 1 0.3781] Jump Over Low Obstacle JOLO
          ;;[1 0.2946 0.274] Lower Forward Trace
          (bind (_returnvalue_6 _outhit_4) (DynamicRaptor|LineTraceDR 0.0 -6e+01 0.0 4.1e+02 "TraceTypeQuery1"))
          ;;[0.4156 1 0.374] Jump on Low Trace Hit (Diff Height Jumps)
          (if (and _returnvalue_6 (.Steep (DynamicRaptor|CheckAngleDR _outhit_4)))
            (if (not _returnvalue_4)
              (if (Variables|DynamicRaptor|GetJumping)
                (bind _outhit_5 (DynamicRaptor|LineTraceDR 4.1e+02 4e+01 -1e+02 0.0 "TraceTypeQuery1"))
                (DynamicRaptor|JumpDR _outhit_5)
                (Variables|DynamicRaptor|SetJumping false)
                (else
                  (Variables|DynamicRaptor|SetJumping true :!label _label))))
            (elif (Character|CanJump)
              (Character|StopJumping)
              (goto _label))))
        (:then_5
          ;[0.9431 1 0.3781] Following Spline Rotation FSR
          ;;[1 0.2946 0.274] Spline
          (DynamicRaptor|SplineDR))))))

(fn SphereTraceDR
  (params (Height :type Float%20%28double-precision%29) (Pitch :type Float%20%28double-precision%29) (Yaw :type Float%20%28double-precision%29) (RightVector :type Float%20%28single-precision%29) (ForwardVector :type Float%20%28single-precision%29) (Distance :type Float%20%28single-precision%29) (Radius :type Float%20%28single-precision%29) (TraceChannel :type ETraceTypeQuery%20Enum :default "TraceTypeQuery1"))
  (bind _returnvalue (Transformation|GetActorForwardVector))
  (bind _returnvalue_2 (Transformation|GetActorLocation))
  (bind _returnvalue_3 (Transformation|GetActorRightVector))
  (bind _returnvalue_4 (Transformation|GetActorRotation))
  (bind (_roll _pitch _yaw) (Math|Rotator|BreakRotator _returnvalue_4))
  (bind (_x _y _z) (Math|Vector|BreakVector _returnvalue_2))
  (bind _returnvalue_5 (* _returnvalue_3 RightVector))
  (bind _returnvalue_6 (* _returnvalue ForwardVector))
  (bind _returnvalue_7 (+ _z Height))
  (bind _returnvalue_8 (Math|Vector|MakeVector _x _y _returnvalue_7))
  (bind _returnvalue_9 (+ _returnvalue_5 _returnvalue_8))
  (bind _returnvalue_10 (+ _returnvalue_6 _returnvalue_9))
  ;[1 1 1] Sphere Trace Coming from RAPTOR, with custom direction/size/distance setting inputs
  (bind (_outhit _returnvalue_11) (Collision|SphereTraceByChannel _returnvalue_10 (+ _returnvalue_10 (* (Math|Rotator|GetRotationXVector (Math|Rotator|MakeRotator _roll (+ _pitch Pitch) (+ _yaw Yaw))) Distance)) Radius TraceChannel false 0 "ForOneFrame"))
  (return _returnvalue_11 _outhit))

(fn LineTraceDR
  (params (Initial%20Forward%20Vector :type Float%20%28double-precision%29) (Initial%20Height :type Float%20%28double-precision%29) (Up%20Vector :type Float%20%28double-precision%29) (Forward%20Vector :type Float%20%28single-precision%29) (TraceChannel :type ETraceTypeQuery%20Enum :default "TraceTypeQuery1"))
  (bind _returnvalue (Transformation|GetActorLocation))
  (bind _returnvalue_2 (Transformation|GetActorForwardVector))
  (bind (_x _y _z) (Math|Vector|BreakVector _returnvalue))
  (bind _returnvalue_3 (* _returnvalue_2 Initial%20Forward%20Vector))
  (bind _returnvalue_4 (+ _z Initial%20Height))
  (bind _returnvalue_5 (Math|Vector|MakeVector _x _y _returnvalue_4))
  (bind _returnvalue_6 (+ _returnvalue_5 _returnvalue_3))
  ;[1 1 1] Line Trace Coming from RAPTOR, with custom direction/distance setting inputs
  (bind (_outhit _returnvalue_7) (Collision|LineTraceByChannel _returnvalue_6 (+ (+ _returnvalue_6 (* (Transformation|GetActorUpVector) Up%20Vector)) (* (Transformation|GetActorForwardVector) Forward%20Vector)) TraceChannel false 0 "ForOneFrame"))
  (return _returnvalue_7 _outhit))

(fn TracesHittingDR
  (params (Hitting :type Boolean))
  ;[1 1 1] If any traces are hitting and rotating character, set to true
  (Utilities|Array|AddUnique (LocalVariables|GetHits) Hitting)
  (bind _array_element (Utilities|Array|ForEachLoopwithBreak (LocalVariables|GetHits) :!label _label)
    (:LoopBody
      (if _array_element
        (Variables|DynamicRaptor|SetHitting true)
        (goto _label Break)
        (else
          (Variables|DynamicRaptor|SetHitting false))))))

(fn CheckRotDR
  (params (Hit :type Hit%20Result%20Structure%20%28by%20ref%29))
  (bind _impactpoint (Collision|BreakHitResult Hit))
  (bind _returnvalue (Transformation|GetActorRotation))
  (bind _returnvalue_2 (Transformation|GetActorLocation))
  (bind _returnvalue_3 (Math|Rotator|FindLookatRotation _returnvalue_2 _impactpoint))
  (bind _returnvalue_4 (Math|Rotator|Delta(Rotator) _returnvalue_3 _returnvalue))
  (bind _yaw (Math|Rotator|BreakRotator _returnvalue_4))
  (return (> _yaw 0.0) _yaw))

(fn CheckAngleDR
  (params (Hit%20Result :type Hit%20Result%20Structure))
  (bind _impactnormal (Collision|BreakHitResult Hit%20Result))
  (return (> (Math|Vector|VectorLengthXY _impactnormal) 0.6) (< (.yaw (Math|Rotator|Delta(Rotator) (Math|Rotator|MakeRotfromZ _impactnormal) (Transformation|GetActorRotation))) 0.0)))

(fn CompareActorDR
  (params (Hit%201 :type Hit%20Result%20Structure%20%28by%20ref%29) (Hit%202 :type Hit%20Result%20Structure) (Hit%203 :type Hit%20Result%20Structure))
  (bind _hitactor (Collision|BreakHitResult Hit%202))
  (bind _hitactor_2 (Collision|BreakHitResult Hit%203))
  (bind _hitactor_3 (Collision|BreakHitResult Hit%201))
  (bind _returnvalue (== _hitactor_3 _hitactor))
  ;[1 1 1] Compare 2 or 3 actors for the same hit actor
  (if (== _hitactor_2 0)
    (return _returnvalue)
    (else
      (return (== _returnvalue (== _hitactor_3 _hitactor_2))))))

(fn TurnSpeedDR
  (params (Hit%20Result :type Hit%20Result%20Structure%20%28by%20ref%29))
  (return (* (Math|Float|MapRangeClamped (Math|Vector|VectorLength (Variables|/Script/Engine.MovementComponent|GetVelocity (Variables|Character|GetCharacterMovement))) 0.0 1.6e+03 0.2 1.0) (Math|Float|MapRangeClamped (.Distance (Collision|BreakHitResult Hit%20Result)) 0.0 6e+02 2.0 0.2))))

(fn RotateDR
  (params (Hit%20Result :type Hit%20Result%20Structure%20%28by%20ref%29) (1.%20RotSpeed :type Float%20%28double-precision%29) (1.%20RotSpeedMult? :type Boolean) (1.%20Invert%20Rot? :type Boolean) (2.%20NearlyEqual? :type Boolean) (2.%20RotIgnoreAmount :type Float%20%28double-precision%29) (2.%20ErrorTolerance :type Float%20%28double-precision%29) (3.%20SlowDown? :type Boolean) (3.%20Slow%20Down%20Decrement :type Float%20%28double-precision%29) (4.%20Dodge? :type Boolean))
  (bind _steep (DynamicRaptor|CheckAngleDR Hit%20Result))
  (bind (_yaw___0 _z__yaw_) (DynamicRaptor|CheckRotDR Hit%20Result))
  (bind _returnvalue (Math|Rotator|MakeRotator 0.0 0.0 1.%20RotSpeed))
  (bind _returnvalue_2 (* 1.%20RotSpeed -1.0))
  (bind _as_player_controller (Variables|Default|GetAs%20Player%20Controller))
  (bind _returnvalue_3 (Math|Float|NearlyEqual(Float) _z__yaw_ 2.%20RotIgnoreAmount 2.%20ErrorTolerance))
  (bind _returnvalue_4 (Math|Rotator|MakeRotator 0.0 0.0 _returnvalue_2))
  (bind _returnvalue_5 (Math|Rotator|SelectRotator _returnvalue_4 _returnvalue _yaw___0))
  (bind _returnvalue_6 (not _returnvalue_3))
  ;[1 1 1] Nearly Equal to the Yaw of Check Rotation
  (if 2.%20NearlyEqual?
    (if _returnvalue_6
      ;[1 1 1] Turn Actor Local Rotation, If angle is steep so you dont turn while going up ramps
      (if _steep :!label _label
        (Transformation|AddActorLocalRotation (* (Math|Rotator|SelectRotator (* _returnvalue_5 (DynamicRaptor|TurnSpeedDR Hit%20Result)) _returnvalue_5 1.%20RotSpeedMult?) (Math|Float|SelectFloat -1.0 1.0 1.%20Invert%20Rot?)) false false)
        ;[1 1 1] Dodge in direction
        (if 4.%20Dodge?
          (if (select 1.%20Invert%20Rot? (not _yaw___0) _yaw___0)
            (Default|DodgeLeft _as_player_controller)
            (else
              (Default|DodgeRight _as_player_controller))))
        ;[1 1 1] Slow down character on tick based on decrement
        (if 3.%20SlowDown?
          (Utilities|SlowDown 0.0 3e+03 3.%20Slow%20Down%20Decrement))
        (return true (.HitActor (Collision|BreakHitResult Hit%20Result)))
        (else
          _)))
    (else
      (goto _label)))
  (if (and (not _returnvalue_6) _steep)
    (Utilities|SlowDown 0.0 3e+03 3.%20Slow%20Down%20Decrement)
    (return false (.HitActor (Collision|BreakHitResult Hit%20Result)))))

(fn JumpDR
  (params (Hit%20Result :type Hit%20Result%20Structure))
  (bind _distance (Collision|BreakHitResult Hit%20Result))
  (bind _returnvalue (Transformation|GetVelocity))
  (bind _charactermovement (Variables|Character|GetCharacterMovement))
  (bind _returnvalue_2 (Math|Vector|VectorLength _returnvalue))
  ;[1 1 1] Character jumps a certain amount based on height of incoming obstacle
  (Variables|/Script/Engine.CharacterMovementComponent|SetJumpZVelocity _charactermovement (* (Variables|/Script/Engine.CharacterMovementComponent|GetJumpZVelocity _charactermovement) (Math|Float|MapRangeClamped _distance 1e+02 0.0 (Math|Float|MapRangeClamped _returnvalue_2 3e+02 1.7e+03 0.8 1.0) (Math|Float|MapRangeClamped _returnvalue_2 3e+02 1.7e+03 1.2 1.6))))
  (if (and (Variables|DynamicRaptor|GetJumping) (> _distance 0.0))
    (Character|Jump)
    (elif (== _distance 0.0)
      (Character|Jump))))

(fn SplineDR
  (bind _returnvalue (Transformation|GetActorLocation))
  (bind _drspline (Variables|DynamicRaptor|GetDRSpline))
  (bind _spline (Variables|/Game/PlayerBPs/Blueprints/BP_DRSpline.BP_DRSpline_C|GetSpline _drspline))
  (bind _returnvalue_2 (Class|SplineComponent|GetDistanceAlongSplineatLocation _spline _returnvalue "World"))
  (bind _returnvalue_3 (Spline|GetRotationatDistanceAlongSpline _spline _returnvalue_2 "World"))
  (Utilities|IsValid (Variables|DynamicRaptor|GetDRSpline)
    (:Is%20Valid
      (if (not (Variables|DynamicRaptor|GetHitting))
        (if (not (Math|Float|NearlyEqual(Float) (.Yaw (Math|Rotator|BreakRotator (Transformation|GetActorRotation))) (.Yaw (Math|Rotator|BreakRotator _returnvalue_3)) 1.0))
          (Transformation|AddActorLocalRotation (Math|Rotator|SelectRotator "0.000000,0.600000,0.000000" "0.000000,-0.600000,0.000000" (< (.Yaw (Math|Rotator|BreakRotator (Math|Rotator|Delta(Rotator) (Transformation|GetActorRotation) _returnvalue_3))) 0.0)) false false))))))

(fn DoSplinesExistDR
  ;[1 1 1] Check If DRSplines exist, add to array and execute function
  (bind _outactors (Actor|GetAllActorsOfClass "/Game/PlayerBPs/Blueprints/BP_DRSpline.BP_DRSpline_C"))
  (bind _output_get (Variables|DynamicRaptor|SetDRSplines _outactors))
  (if (> (Utilities|Array|Length _output_get) 0)
    (DynamicRaptor|GetClosestSplineDR)
    (Utilities|Time|SetTimerbyFunctionName 0 "GetClosestSplineDR" 5.0 true)))

(fn GetClosestSplineDR
  (bind _returnvalue (Transformation|GetActorLocation))
  (bind _drsplines (Variables|DynamicRaptor|GetDRSplines))
  (bind _returnvalue_2 (Actor|FindNearestActor _returnvalue _drsplines))
  (bind _asbp_drspline (Utilities|Casting|CastToBP_DRSpline _returnvalue_2))
  (bind _spline (Variables|/Game/PlayerBPs/Blueprints/BP_DRSpline.BP_DRSpline_C|GetSpline _asbp_drspline))
  ;[1 1 1] Get Spline closest to player actor, get actors distance along spline, if above 5000 units of distance, dismiss spline and follow nothing
  (Utilities|IsValid _returnvalue_2
    (:Is%20Valid
      (if (> (Math|Vector|Distance(Vector) (Spline|GetLocationatDistanceAlongSpline _spline (Class|SplineComponent|GetDistanceAlongSplineatLocation _spline _returnvalue "World") "World") (Transformation|GetActorLocation)) 5e+03)
        (Variables|DynamicRaptor|SetDRSpline 0)
        (else
          (Variables|DynamicRaptor|SetDRSpline _asbp_drspline))))))

(event EventOnLanded
  (params (Hit :type Hit%20Result%20Structure%20%28by%20ref%29))
  (Game|Feedback|ClientStartCameraShake (Game|GetPlayerController 0) "/Game/PlayerBPs/Other/JumpShake.JumpShake_C" 1.0 "CameraLocal" "0, 0, 0")
  (Variables|/Script/Engine.CharacterMovementComponent|SetJumpZVelocity (Variables|Character|GetCharacterMovement) 3.5e+02)
  (Variables|DynamicRaptor|SetJumping true))

(event EventOnJumped
  (Game|Feedback|ClientStartCameraShake (Game|GetPlayerController 0) "/Game/PlayerBPs/Other/JumpShake.JumpShake_C" 1.0 "CameraLocal" "0, 0, 0"))

(event Collision|EventHit
  (params (MyComp :type Primitive%20Component%20Object%20Reference) (Other :type Actor%20Object%20Reference) (OtherComp :type Primitive%20Component%20Object%20Reference) (bSelfMoved :type Boolean) (HitLocation :type Vector :default "0, 0, 0") (HitNormal :type Vector :default "0, 0, 0") (NormalImpulse :type Vector :default "0, 0, 0") (Hit :type Hit%20Result%20Structure%20%28by%20ref%29))
  (bind _bool (Class|BPIInteraction|CheckMatchingGameplayTag(Message) Other "(GameplayTags=((TagName=\"World.Obstacle\")))"))
  (if _bool
    (Game|Feedback|ClientStartCameraShake (Game|GetPlayerController 0) "/Game/PlayerBPs/Other/HitShake.HitShake_C" 1.0 "CameraLocal" "0, 0, 0")))

(event Custom|HealOT
  (bind _returnvalue (Utilities|Time|SetTimerbyFunctionName 0 "RecoverHealth" 0.016667 true))
  (if (== (Variables|Default|GetHealth) 1e+02)
    (Utilities|Time|ClearandInvalidateTimerbyHandle _returnvalue)))

(event Game|Damage|EventAnyDamage
  (params (Damage :type Float%20%28single-precision%29) (DamageType :type Damage%20Type%20Object%20Reference) (InstigatedBy :type Controller%20Object%20Reference) (DamageCauser :type Actor%20Object%20Reference))
  (Variables|Default|SetHealth (Math|Float|Clamp(Float) (- (Variables|Default|GetHealth) Damage) 0.0 1e+02))
  (Utilities|Time|ClearandInvalidateTimerbyHandle (stale Custom|HealOT _returnvalue))
  (Utilities|Time|SetTimerbyEvent (delegate Custom|HealOT) 3.0))

(event EventBeginPlay
  (bind _asbp_player_controller (Utilities|Casting|CastToBP_PlayerController (Pawn|GetController)))
  (bind _output_get (Variables|Default|SetAs%20Player%20Controller _asbp_player_controller))
  (Utilities|IsValid (PlayerController|LocalPlayerSubsystems|GetEnhancedInputLocalPlayerSubsystem _output_get)
    (:Is%20Valid
      (Input|AddMappingContext (PlayerController|LocalPlayerSubsystems|GetEnhancedInputLocalPlayerSubsystem _output_get) "/Game/PlayerBPs/Input/IMC_Default.IMC_Default" 0 "(bIgnoreAllPressedKeysUntilRelease=True,bForceImmediately=False,bNotifyUserSettings=False)")
      (Input|EnableInput (Game|GetPlayerController 0))
      (CallFunction|HUD)
      (Physics|SetSimulatePhysics (Variables|Collision|GetCapsuleComponent) false)
      (bind _asbp_player_camera_manager (Utilities|Casting|CastToBP_PlayerCameraManager (Variables|/Script/Engine.PlayerController|GetPlayerCameraManager (Game|GetPlayerController 0))))
      (Variables|/Game/PlayerBPs/Blueprints/BP_PlayerCameraManager.BP_PlayerCameraManager_C|SetChar _asbp_player_camera_manager self)
      (DynamicRaptor|DoSplinesExistDR))))

(event Custom|Cooldown
  (if (Math|Boolean|ORBoolean (Input|EnhancedActionValues|GetIA_MoveReset) (not (Character|CanJump)) (> (Math|Vector|VectorLength (Transformation|GetVelocity)) 1.6e+03))
    ;[1 1 1] Activates Handle, initiating cooldown. Invalidates after 1 second to re-enable DRS
    (bind _returnvalue (Utilities|Time|SetTimerbyEvent (delegate Custom|CooldownTimer) 1.0))
    (Variables|DynamicRaptor|SetDRCDTimerHandle _returnvalue)))

(event Custom|CooldownTimer
  ;[1 1 1] Activates Handle, initiating cooldown. Invalidates after 1 second to re-enable DRS
  (Utilities|Time|ClearandInvalidateTimerbyHandle (Variables|DynamicRaptor|GetDRCDTimerHandle)))