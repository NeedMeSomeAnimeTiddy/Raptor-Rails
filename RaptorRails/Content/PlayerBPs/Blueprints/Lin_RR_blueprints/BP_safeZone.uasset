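; BP_safeZone is a moving zone actor that travels along a spline path and reacts when the player enters it.
; On BeginPlay it finds the Bp_Path actor and starts a Timeline whose alpha maps to distance along that spline, setting location and rotation each update.
; Its Box overlap checks for the "Player" tag and only prints a "follow the train!" message, with no protection logic.
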(event OnComponentBeginOverlap(Box)
  (params (OverlappedComponent :type Primitive%20Component%20Object%20Reference) (OtherActor :type Actor%20Object%20Reference) (OtherComp :type Primitive%20Component%20Object%20Reference) (OtherBodyIndex :type Integer) (bFromSweep :type Boolean) (SweepResult :type Hit%20Result%20Structure%20%28by%20ref%29))
  (if (Actor|ActorHasTag OtherActor "Player")
    (Development|PrintString "follow the train!")))

(event Custom|startmoving
  (bind _alpha (Timeline|Timeline Play)
    (:Update
      (Transformation|SetActorLocationAndRotation (.location (Spline|GetTransformatDistanceAlongSpline (Variables|/Game/PlayerBPs/Blueprints/Lin_RR_blueprints/Bp_Path.Bp_Path_C|GetSpline (Variables|Default|Getpath)) (Math|Float|Lerp 0.0 (Spline|GetSplineLength (Variables|/Game/PlayerBPs/Blueprints/Lin_RR_blueprints/Bp_Path.Bp_Path_C|GetSpline (Variables|Default|Getpath))) _alpha) "World" false)) (.rotation (Spline|GetTransformatDistanceAlongSpline (Variables|/Game/PlayerBPs/Blueprints/Lin_RR_blueprints/Bp_Path.Bp_Path_C|GetSpline (Variables|Default|Getpath)) (Math|Float|Lerp 0.0 (Spline|GetSplineLength (Variables|/Game/PlayerBPs/Blueprints/Lin_RR_blueprints/Bp_Path.Bp_Path_C|GetSpline (Variables|Default|Getpath))) _alpha) "World" false))))))

(event EventBeginPlay
  (bind _returnvalue (Actor|GetActorOfClass "/Game/PlayerBPs/Blueprints/Lin_RR_blueprints/Bp_Path.Bp_Path_C"))
  (Variables|Default|Setpath _returnvalue)
  (CallFunction|Startmoving))

(fn ConstructionScript)