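; Player controller that drives BP_DinoRider, a constantly forward-moving mounted shooter character, through Enhanced Input.
; Handles strafing, dodging, variable jumps, look, and speed control or boost, with a looping timer easing speed back to cruise.
; Timeline-driven aiming gates sphere-trace shooting with limited ammo and timed reload, while timed slow-mo uses global time dilation.
; Gameplay tags track states and gate actions; the turn timeline is marked not working.
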(fn ConstructionScript)

(fn ShootLineTrace
  (bind _as_bp_dino_rider (Variables|Default|GetAs%20BP%20Dino%20Rider))
  (bind _gameplaytags (Variables|Default|GetGameplayTags))
  (bind _camera (Variables|/Game/PlayerBPs/Blueprints/BP_DinoRider.BP_DinoRider_C|GetCamera _as_bp_dino_rider))
  (bind _returnvalue (Transformation|GetWorldLocation _camera))
  (bind (_outhit _returnvalue_2) (Collision|SphereTraceByChannel _returnvalue (+ _returnvalue (* (Math|Vector|GetForwardVector _camera) 2e+04)) 1e+01 "TraceTypeQuery3" false 0 "Persistent"))
  (if _returnvalue_2
    (GameplayTags|AddGameplayTag _gameplaytags "(TagName=\"Player.Hit\")" :!class /Script/GameplayTags.BlueprintGameplayTagLibrary)
    (Variables|Default|SetHit%20Actor (.HitActor (Collision|BreakHitResult _outhit)))
    (Variables|Default|SetHit%20Bone%20Name (.HitBoneName (Collision|BreakHitResult _outhit)))
    (else
      (GameplayTags|RemoveGameplayTag _gameplaytags "(TagName=\"Player.Hit\")" :!class /Script/GameplayTags.BlueprintGameplayTagLibrary)
      (Variables|Default|SetHit%20Actor 0)
      (Variables|Default|SetHit%20Bone%20Name "None")))
  (Variables|Default|SetBullets (Math|Integer|Clamp(Integer) (- (Variables|Default|GetBullets) 1) 0 6)))

(fn SpeedUp
  (bind _as_bp_dino_rider (Variables|Default|GetAs%20BP%20Dino%20Rider))
  (bind _charactermovement (Variables|/Script/Engine.Character|GetCharacterMovement _as_bp_dino_rider))
  (Variables|/Script/Engine.CharacterMovementComponent|SetMaxWalkSpeed _charactermovement (Math|Float|Clamp(Float) (Math|Interpolation|FInterpTo (Variables|/Script/Engine.CharacterMovementComponent|GetMaxWalkSpeed _charactermovement) (+ (Variables|/Script/Engine.CharacterMovementComponent|GetMaxWalkSpeed _charactermovement) 4e+02) (Variables|Default|GetDelta%20Seconds) 1.0) 2e+03 2.5e+03)))

(fn SlowDown
  (bind _as_bp_dino_rider (Variables|Default|GetAs%20BP%20Dino%20Rider))
  (bind _charactermovement (Variables|/Script/Engine.Character|GetCharacterMovement _as_bp_dino_rider))
  (Variables|/Script/Engine.CharacterMovementComponent|SetMaxWalkSpeed _charactermovement (Math|Float|Clamp(Float) (Math|Interpolation|FInterpTo (Variables|/Script/Engine.CharacterMovementComponent|GetMaxWalkSpeed _charactermovement) (- (Variables|/Script/Engine.CharacterMovementComponent|GetMaxWalkSpeed _charactermovement) 2e+02) (Variables|Default|GetDelta%20Seconds) 3.0) 0.0 2e+03)))

(fn RegulateSpeed
  (bind _as_bp_dino_rider (Variables|Default|GetAs%20BP%20Dino%20Rider))
  (bind _charactermovement (Variables|/Script/Engine.Character|GetCharacterMovement _as_bp_dino_rider))
  (bind _output_get (Variables|/Script/Engine.CharacterMovementComponent|SetMaxWalkSpeed _charactermovement (Math|Interpolation|FInterpTo (Variables|/Script/Engine.CharacterMovementComponent|GetMaxWalkSpeed _charactermovement) 2e+03 (Variables|Default|GetDelta%20Seconds) 1.0)))
  (if (== _output_get 2e+03)
    (Class|KismetSystemLibrary|PauseTimer 0 "RegulateSpeed")))

(fn Boost
  (bind _as_bp_dino_rider (Variables|Default|GetAs%20BP%20Dino%20Rider))
  (bind _charactermovement (Variables|/Script/Engine.Character|GetCharacterMovement _as_bp_dino_rider))
  (Class|KismetSystemLibrary|PauseTimer 0 "RegulateSpeed")
  (GameplayTags|AddGameplayTag (Variables|Default|GetGameplayTags) "(TagName=\"Player.State.Boosting\")" :!class /Script/GameplayTags.BlueprintGameplayTagLibrary)
  (Variables|/Script/Engine.CharacterMovementComponent|SetMaxWalkSpeed _charactermovement (Math|Float|Clamp(Float) (Math|Interpolation|FInterpTo (Variables|/Script/Engine.CharacterMovementComponent|GetMaxWalkSpeed _charactermovement) (+ (Variables|/Script/Engine.CharacterMovementComponent|GetMaxWalkSpeed _charactermovement) 1.5e+03) (Variables|Default|GetDelta%20Seconds) 1e+02) 1.5e+03 4.5e+03)))

(fn SelectJumpVel
  (bind _as_bp_dino_rider (Variables|Default|GetAs%20BP%20Dino%20Rider))
  (bind _charactermovement (Variables|/Script/Engine.Character|GetCharacterMovement _as_bp_dino_rider))
  (bind _velocity (Variables|/Script/Engine.MovementComponent|GetVelocity _charactermovement))
  (bind _returnvalue (Math|Vector|VectorLength _velocity))
  (return (select (< _returnvalue 5e+01) 3.5e+02 (* _returnvalue 0.3))))

(fn CheckMatchingGameplayTag
  (params (Tag%20Container :type Gameplay%20Tag%20Container%20Structure))
  (return (|MultiCompareGameplayTagContainer Tag%20Container (Variables|Default|GetGameplayTags))))

(event Custom|ResetJump
  (bind _as_bp_dino_rider (Variables|Default|GetAs%20BP%20Dino%20Rider))
  (bind _charactermovement (Variables|/Script/Engine.Character|GetCharacterMovement _as_bp_dino_rider))
  (Utilities|FlowControl|DoOnce false) ; enters at Reset
)

(event Input|EnhancedActionEvents|EnhancedInputActionIA_Jump
  (params (ActionValue :type Boolean) (ElapsedSeconds :type Float%20%28double-precision%29) (TriggeredSeconds :type Float%20%28double-precision%29) (InputAction :type Input%20Action%20Object%20Reference :default "/Game/PlayerBPs/Input/Actions/IA_Jump.IA_Jump"))
  (bind _as_bp_dino_rider (Variables|Default|GetAs%20BP%20Dino%20Rider))
  (bind _charactermovement (Variables|/Script/Engine.Character|GetCharacterMovement _as_bp_dino_rider))
  (:Started
    (if (Character|CanJump _as_bp_dino_rider)
      (Utilities|FlowControl|DoOnce false
        (:Completed
          (bind _value (Timeline|JumpTL PlayFromStart)
            (:Update
              (Variables|/Script/Engine.CharacterMovementComponent|SetGravityScale _charactermovement _value)
              (Variables|/Script/Engine.CharacterMovementComponent|SetJumpZVelocity _charactermovement (CallFunction|SelectJumpVel))
              (Character|Jump _as_bp_dino_rider)))))))
  (:Completed
    (Utilities|FlowControl|Sequence
      (:then_0
        (Timeline|JumpTL Stop))
      (:then_1
        (Variables|/Script/Engine.CharacterMovementComponent|SetGravityScale _charactermovement (Variables|Default|GetDefaultGrav))
        (Character|StopJumping _as_bp_dino_rider)
        (CallFunction|ResetJump)))))

(event Custom|ResetBoost
  (Utilities|FlowControl|DoOnce false) ; enters at Reset
)

(event Custom|SlowSpeed
  (bind _returnvalue (Utilities|Time|SetTimerbyFunctionName 0 "RegulateSpeed" 0.016667 true))
  (Utilities|Time|UnpauseTimerbyHandle _returnvalue)
  (GameplayTags|RemoveGameplayTag (Variables|Default|GetGameplayTags) "(TagName=\"Player.State.Boosting\")" :!class /Script/GameplayTags.BlueprintGameplayTagLibrary))

(event Input|EnhancedActionEvents|EnhancedInputActionIA_Boost
  (params (ActionValue :type Boolean) (ElapsedSeconds :type Float%20%28double-precision%29) (TriggeredSeconds :type Float%20%28double-precision%29) (InputAction :type Input%20Action%20Object%20Reference :default "/Game/PlayerBPs/Input/Actions/IA_Boost.IA_Boost"))
  (:Started
    (Utilities|FlowControl|DoOnce false
      (:Completed
        (CallFunction|StopAiming)
        (Utilities|Time|SetTimerbyEvent (delegate Custom|ResetBoost) 5.0)
        (CallFunction|Boost)
        (Utilities|Time|SetTimerbyEvent (delegate Custom|SlowSpeed) 2.0)))))

(event Custom|Reloading
  (Variables|Default|SetBullets 6)
  (CallFunction|ResetReload))

(event Custom|ResetReload
  (Utilities|FlowControl|DoOnce false) ; enters at Reset
)

(event Input|EnhancedActionEvents|EnhancedInputActionIA_Reload
  (params (ActionValue :type Boolean) (ElapsedSeconds :type Float%20%28double-precision%29) (TriggeredSeconds :type Float%20%28double-precision%29) (InputAction :type Input%20Action%20Object%20Reference :default "/Game/PlayerBPs/Input/Actions/IA_Reload.IA_Reload"))
  (:Started
    (Utilities|FlowControl|DoOnce false
      (:Completed
        (Utilities|Time|SetTimerbyEvent (delegate Custom|Reloading) 3.0)))))

(event Custom|DodgeRight
  (bind _as_bp_dino_rider (Variables|Default|GetAs%20BP%20Dino%20Rider))
  (Utilities|FlowControl|DoOnce false :!label _label
    (:Completed
      (bind _newtrack_0 (Timeline|DodgeTL PlayFromStart)
        (:Update
          (Class|Actor|AddActorLocalTransform _as_bp_dino_rider (Math|Transform|MakeTransform (Math|Vector|MakeVector 0.0 (Math|Float|Lerp 0.0 5.0 _newtrack_0) 0.0) "0, 0, 0" "1.000000,1.000000,1.000000") false false))
        (:Finished
          (Utilities|FlowControl|Sequence
            (:then_0
              (Utilities|FlowControl|DoOnce false) ; enters at Reset
            )
            (:then_1
              (goto _label Reset))
            (:then_2
              (Utilities|FlowControl|DoOnce false) ; enters at Reset
            )))))))

(event Custom|DodgeLeft
  (bind _as_bp_dino_rider (Variables|Default|GetAs%20BP%20Dino%20Rider))
  (Utilities|FlowControl|DoOnce false :!label _label
    (:Completed
      (bind _newtrack_0 (Timeline|DodgeTL2 PlayFromStart)
        (:Update
          (Class|Actor|AddActorLocalTransform _as_bp_dino_rider (Math|Transform|MakeTransform (Math|Vector|MakeVector 0.0 (Math|Float|Lerp 0.0 -5.0 _newtrack_0) 0.0) "0, 0, 0" "1.000000,1.000000,1.000000") false false))
        (:Finished
          (Utilities|FlowControl|Sequence
            (:then_0
              (Utilities|FlowControl|DoOnce false) ; enters at Reset
            )
            (:then_1
              (Utilities|FlowControl|DoOnce false) ; enters at Reset
            )
            (:then_2
              (goto _label Reset))))))))

(event Custom|TurnTL
  ;[1 1 1] NOT WORKING
  (bind _newtrack_0 (Timeline|Timeline_0 Play)
    (:Update
      (if (Input|EnhancedActionValues|GetIA_MoveReset)
        (Variables|Default|SetRot (Math|Rotator|SelectRotator (Math|Rotator|MakeRotator 0.0 0.0 _newtrack_0) (* (Math|Rotator|MakeRotator 0.0 0.0 _newtrack_0) -1.0) false))
        (else
          (Utilities|FlowControl|DoOnce false
            (:Completed
              (CallFunction|ResetTurn)
              (CallFunction|ResetResetTurn))))))))

(event Custom|ResetTurn
  ;[1 1 1] NOT WORKING
  (bind _newtrack_0 (Timeline|Timeline_0 SetNewTime)
    (:Update
      (if (Input|EnhancedActionValues|GetIA_MoveReset)
        (Variables|Default|SetRot (Math|Rotator|SelectRotator (Math|Rotator|MakeRotator 0.0 0.0 _newtrack_0) (* (Math|Rotator|MakeRotator 0.0 0.0 _newtrack_0) -1.0) false))
        (else
          (Utilities|FlowControl|DoOnce false
            (:Completed
              (CallFunction|ResetTurn)
              (CallFunction|ResetResetTurn))))))))

(event Custom|ResetResetTurn
  ;[1 1 1] NOT WORKING
  (Utilities|FlowControl|DoOnce false) ; enters at Reset
)

(event Input|EnhancedActionEvents|EnhancedInputActionIA_Dodge
  (params (ActionValue :type Boolean) (ElapsedSeconds :type Float%20%28double-precision%29) (TriggeredSeconds :type Float%20%28double-precision%29) (InputAction :type Input%20Action%20Object%20Reference :default "/Game/PlayerBPs/Input/Actions/IA_Dodge.IA_Dodge"))
  (bind _as_bp_dino_rider (Variables|Default|GetAs%20BP%20Dino%20Rider))
  (Utilities|FlowControl|DoOnce false :!label _label
    (:Completed
      (Math|Float|CompareFloat (.x (Input|EnhancedActionValues|GetIA_Move)) 0.0
        (:>
          (bind _newtrack_0 (Timeline|DodgeTL PlayFromStart)
            (:Update
              (Class|Actor|AddActorLocalTransform _as_bp_dino_rider (Math|Transform|MakeTransform (Math|Vector|MakeVector 0.0 (Math|Float|Lerp 0.0 5.0 _newtrack_0) 0.0) "0, 0, 0" "1.000000,1.000000,1.000000") false false))
            (:Finished
              (Utilities|FlowControl|Sequence :!label _label_2
                (:then_0
                  (goto _label Reset))
                (:then_1
                  (Utilities|FlowControl|DoOnce false) ; enters at Reset
                )
                (:then_2
                  (Utilities|FlowControl|DoOnce false) ; enters at Reset
                )))))
        (:==
          (goto _label_2))
        (:<
          (bind _newtrack_0_2 (Timeline|DodgeTL2 PlayFromStart)
            (:Update
              (Class|Actor|AddActorLocalTransform _as_bp_dino_rider (Math|Transform|MakeTransform (Math|Vector|MakeVector 0.0 (Math|Float|Lerp 0.0 -5.0 _newtrack_0_2) 0.0) "0, 0, 0" "1.000000,1.000000,1.000000") false false))
            (:Finished
              (goto _label_2))))))))

(event Input|EnhancedActionEvents|EnhancedInputActionIA_Move
  (params (ActionValue :type Vector%202D%20Structure) (ElapsedSeconds :type Float%20%28double-precision%29) (TriggeredSeconds :type Float%20%28double-precision%29) (InputAction :type Input%20Action%20Object%20Reference :default "/Game/PlayerBPs/Input/Actions/IA_Move.IA_Move"))
  (bind _as_bp_dino_rider (Variables|Default|GetAs%20BP%20Dino%20Rider))
  (bind _returnvalue (Transformation|GetActorRightVector _as_bp_dino_rider))
  (if (not (AI|Components|NavMovement|IsFalling (Variables|/Script/Engine.Character|GetCharacterMovement (Variables|Default|GetAs%20BP%20Dino%20Rider))))
    (Pawn|Input|AddMovementInput _as_bp_dino_rider (Math|Vector|SelectVector _returnvalue (* _returnvalue -1.0) (> (.x ActionValue) (.y ActionValue))) 0.02 false)))

(event Input|EnhancedActionEvents|EnhancedInputActionIA_SpeedAdjust
  (params (ActionValue :type Float%20%28double-precision%29) (ElapsedSeconds :type Float%20%28double-precision%29) (TriggeredSeconds :type Float%20%28double-precision%29) (InputAction :type Input%20Action%20Object%20Reference :default "/Game/PlayerBPs/Input/Actions/IA_SpeedAdjust.IA_SpeedAdjust"))
  (:Triggered
    (if (not (GameplayTags|HasTag (Variables|Default|GetGameplayTags) "(TagName=\"Player.State.Slowed\")"))
      (if (not (GameplayTags|HasTag (Variables|Default|GetGameplayTags) "(TagName=\"Player.State.Boosting\")"))
        (if (not (GameplayTags|HasTag (Variables|Default|GetGameplayTags) "(TagName=\"Player.State.Avoiding\")"))
          (Math|Float|CompareFloat ActionValue 0.0
            (:>
              (CallFunction|SpeedUp))
            (:<
              (CallFunction|SlowDown)))
          (Class|KismetSystemLibrary|PauseTimer 0 "RegulateSpeed")))))
  (:Completed
    (if (not (GameplayTags|HasTag (Variables|Default|GetGameplayTags) "(TagName=\"Player.State.Avoiding\")"))
      (bind _returnvalue (Utilities|Time|SetTimerbyFunctionName 0 "RegulateSpeed" 0.016667 true))
      (Utilities|Time|UnpauseTimerbyHandle _returnvalue))))

(event Custom|ResetShot
  (Utilities|FlowControl|DoOnce false) ; enters at Reset
)

(event Input|EnhancedActionEvents|EnhancedInputActionIA_Shoot
  (params (ActionValue :type Boolean) (ElapsedSeconds :type Float%20%28double-precision%29) (TriggeredSeconds :type Float%20%28double-precision%29) (InputAction :type Input%20Action%20Object%20Reference :default "/Game/PlayerBPs/Input/Actions/IA_Shoot.IA_Shoot"))
  (:Started
    (Utilities|FlowControl|DoOnce false
      (:Completed
        (Utilities|Time|SetTimerbyEvent (delegate Custom|ResetShot) 0.3)
        (if (> (Variables|Default|GetBullets) 0)
          (if (GameplayTags|HasTag (Variables|Default|GetGameplayTags) "(TagName=\"Player.State.Aiming\")")
            (Niagara|ResetSystem (Variables|/Game/PlayerBPs/Blueprints/BP_DinoRider.BP_DinoRider_C|GetBulletTracer (Variables|Default|GetAs%20BP%20Dino%20Rider)))
            (CallFunction|ShootLineTrace)
            (if (GameplayTags|HasTag (Variables|Default|GetGameplayTags) "(TagName=\"Player.Hit\")")
              (Class|BPIInteraction|Shot(Message) (Variables|Default|GetHit%20Actor) (Variables|Default|GetHit%20Bone%20Name))))
          (else
            (Audio|PlaySound2D 0 1.0 1.0 0.0 0 0)))))))

(event Custom|SlowMoTime
  (bind _as_bp_dino_rider (Variables|Default|GetAs%20BP%20Dino%20Rider))
  (bind _springarm (Variables|/Game/PlayerBPs/Blueprints/BP_DinoRider.BP_DinoRider_C|GetSpringArm _as_bp_dino_rider))
  (Utilities|Time|SetGlobalTimeDilation 1.0)
  (Utilities|Time|ClearandInvalidateTimerbyHandle (stale Input|EnhancedActionEvents|EnhancedInputActionIA_TimeDilation _returnvalue))
  (CallFunction|ResetSlowMo)
  (Variables|Default|SetSens 1.0)
  (Variables|/Script/Engine.SpringArmComponent|SetbEnableCameraRotationLag _springarm false)
  (Variables|/Script/Engine.SpringArmComponent|SetCameraRotationLagSpeed _springarm 0.0))

(event Custom|ResetSlowMo
  (bind _gameplaytags (Variables|Default|GetGameplayTags))
  (bind _as_bp_dino_rider (Variables|Default|GetAs%20BP%20Dino%20Rider))
  (bind _springarm (Variables|/Game/PlayerBPs/Blueprints/BP_DinoRider.BP_DinoRider_C|GetSpringArm _as_bp_dino_rider))
  (if (Input|EnhancedActionValues|GetIA_Aim)
    _
    (else
      (CallFunction|StopAiming)))
  (GameplayTags|RemoveGameplayTag _gameplaytags "(TagName=\"Player.State.Slowmo\")" :!class /Script/GameplayTags.BlueprintGameplayTagLibrary)
  (Utilities|FlowControl|DoOnce false) ; enters at Reset
)

(event Input|EnhancedActionEvents|EnhancedInputActionIA_TimeDilation
  (params (ActionValue :type Boolean) (ElapsedSeconds :type Float%20%28double-precision%29) (TriggeredSeconds :type Float%20%28double-precision%29) (InputAction :type Input%20Action%20Object%20Reference :default "/Game/PlayerBPs/Input/Actions/IA_TimeDilation.IA_TimeDilation"))
  (bind _gameplaytags (Variables|Default|GetGameplayTags))
  (bind _as_bp_dino_rider (Variables|Default|GetAs%20BP%20Dino%20Rider))
  (bind _springarm (Variables|/Game/PlayerBPs/Blueprints/BP_DinoRider.BP_DinoRider_C|GetSpringArm _as_bp_dino_rider))
  (:Started
    (GameplayTags|AddGameplayTag _gameplaytags "(TagName=\"Player.State.Slowmo\")" :!class /Script/GameplayTags.BlueprintGameplayTagLibrary)
    (Utilities|FlowControl|DoOnce false
      (:Completed
        (if (GameplayTags|HasTag _gameplaytags "(TagName=\"Player.State.Aiming\")")
          _
          (else
            (CallFunction|Aimin)))
        (Utilities|FlowControl|Sequence
          (:then_0
            (Utilities|Time|SetGlobalTimeDilation 0.25)
            (Variables|Default|SetSens 0.5)
            (Variables|/Script/Engine.SpringArmComponent|SetbEnableCameraRotationLag _springarm true)
            (Variables|/Script/Engine.SpringArmComponent|SetCameraRotationLagSpeed _springarm 2e+01))
          (:then_1
            (bind _returnvalue (Utilities|Time|SetTimerbyEvent (delegate Custom|SlowMoTime) 2.0))))))))

(event Custom|AimIn
  (bind _gameplaytags (Variables|Default|GetGameplayTags))
  (bind _as_bp_dino_rider (Variables|Default|GetAs%20BP%20Dino%20Rider))
  (bind _camera (Variables|/Game/PlayerBPs/Blueprints/BP_DinoRider.BP_DinoRider_C|GetCamera _as_bp_dino_rider))
  (bind _reticleref (Variables|/Game/PlayerBPs/Blueprints/BP_DinoRider.BP_DinoRider_C|GetReticleREF _as_bp_dino_rider))
  (GameplayTags|AddGameplayTag _gameplaytags "(TagName=\"Player.State.Aiming\")" :!class /Script/GameplayTags.BlueprintGameplayTagLibrary)
  (bind _track (Timeline|Timeline Play)
    (:Update
      (if (GameplayTags|HasTag _gameplaytags "(TagName=\"Player.State.Aiming\")")
        (Camera|SetFieldOfView _camera (Math|Float|Lerp 9e+01 5e+01 _track))
        (Transformation|SetRelativeLocation _camera (Math|Vector|Lerp(Vector) "0, 0, 0" "0.000000,60.000000,0.000000" _track) false false)
        (UserInterface|Viewport|AddtoViewport _reticleref 0)
        (Variables|Default|SetSens 0.7)
        (else
          (Camera|SetFieldOfView _camera (Math|Float|Lerp 9e+01 5e+01 _track))
          (Transformation|SetRelativeLocation _camera (Math|Vector|Lerp(Vector) "0, 0, 0" "0.000000,60.000000,0.000000" _track) false false)
          (Widget|RemovefromParent _reticleref)
          (Variables|Default|SetSens 1.0))))))

(event Custom|StopAiming
  (bind _gameplaytags (Variables|Default|GetGameplayTags))
  (bind _as_bp_dino_rider (Variables|Default|GetAs%20BP%20Dino%20Rider))
  (bind _camera (Variables|/Game/PlayerBPs/Blueprints/BP_DinoRider.BP_DinoRider_C|GetCamera _as_bp_dino_rider))
  (bind _reticleref (Variables|/Game/PlayerBPs/Blueprints/BP_DinoRider.BP_DinoRider_C|GetReticleREF _as_bp_dino_rider))
  (GameplayTags|RemoveGameplayTag _gameplaytags "(TagName=\"Player.State.Aiming\")" :!class /Script/GameplayTags.BlueprintGameplayTagLibrary)
  (bind _track (Timeline|Timeline Reverse)
    (:Update
      (if (GameplayTags|HasTag _gameplaytags "(TagName=\"Player.State.Aiming\")")
        (Camera|SetFieldOfView _camera (Math|Float|Lerp 9e+01 5e+01 _track))
        (Transformation|SetRelativeLocation _camera (Math|Vector|Lerp(Vector) "0, 0, 0" "0.000000,60.000000,0.000000" _track) false false)
        (UserInterface|Viewport|AddtoViewport _reticleref 0)
        (Variables|Default|SetSens 0.7)
        (else
          (Camera|SetFieldOfView _camera (Math|Float|Lerp 9e+01 5e+01 _track))
          (Transformation|SetRelativeLocation _camera (Math|Vector|Lerp(Vector) "0, 0, 0" "0.000000,60.000000,0.000000" _track) false false)
          (Widget|RemovefromParent _reticleref)
          (Variables|Default|SetSens 1.0))))))

(event Input|EnhancedActionEvents|EnhancedInputActionIA_Aim
  (params (ActionValue :type Boolean) (ElapsedSeconds :type Float%20%28double-precision%29) (TriggeredSeconds :type Float%20%28double-precision%29) (InputAction :type Input%20Action%20Object%20Reference :default "/Game/PlayerBPs/Input/Actions/IA_Aim.IA_Aim"))
  (bind _gameplaytags (Variables|Default|GetGameplayTags))
  (bind _as_bp_dino_rider (Variables|Default|GetAs%20BP%20Dino%20Rider))
  (bind _camera (Variables|/Game/PlayerBPs/Blueprints/BP_DinoRider.BP_DinoRider_C|GetCamera _as_bp_dino_rider))
  (bind _reticleref (Variables|/Game/PlayerBPs/Blueprints/BP_DinoRider.BP_DinoRider_C|GetReticleREF _as_bp_dino_rider))
  (:Started
    (GameplayTags|AddGameplayTag _gameplaytags "(TagName=\"Player.State.Aiming\")" :!class /Script/GameplayTags.BlueprintGameplayTagLibrary)
    (bind _track (Timeline|Timeline Play)
      (:Update
        (if (GameplayTags|HasTag _gameplaytags "(TagName=\"Player.State.Aiming\")")
          (Camera|SetFieldOfView _camera (Math|Float|Lerp 9e+01 5e+01 _track))
          (Transformation|SetRelativeLocation _camera (Math|Vector|Lerp(Vector) "0, 0, 0" "0.000000,60.000000,0.000000" _track) false false)
          (UserInterface|Viewport|AddtoViewport _reticleref 0)
          (Variables|Default|SetSens 0.7)
          (else
            (Camera|SetFieldOfView _camera (Math|Float|Lerp 9e+01 5e+01 _track))
            (Transformation|SetRelativeLocation _camera (Math|Vector|Lerp(Vector) "0, 0, 0" "0.000000,60.000000,0.000000" _track) false false)
            (Widget|RemovefromParent _reticleref)
            (Variables|Default|SetSens 1.0))))))
  (:Completed
    (GameplayTags|RemoveGameplayTag _gameplaytags "(TagName=\"Player.State.Aiming\")" :!class /Script/GameplayTags.BlueprintGameplayTagLibrary)
    (Timeline|Timeline Reverse)))

(event Input|EnhancedActionEvents|EnhancedInputActionIA_Look
  (params (ActionValue :type Vector%202D%20Structure) (ElapsedSeconds :type Float%20%28double-precision%29) (TriggeredSeconds :type Float%20%28double-precision%29) (InputAction :type Input%20Action%20Object%20Reference :default "/Game/PlayerBPs/Input/Actions/IA_Look.IA_Look"))
  (bind _sens (Variables|Default|GetSens))
  (bind _as_bp_dino_rider (Variables|Default|GetAs%20BP%20Dino%20Rider))
  (Pawn|Input|AddControllerYawInput _as_bp_dino_rider (* (.x ActionValue) _sens))
  (Pawn|Input|AddControllerPitchInput _as_bp_dino_rider (* (.y ActionValue) _sens)))

(event EventTick
  (params (DeltaSeconds :type Float%20%28single-precision%29))
  (bind _as_bp_dino_rider (Variables|Default|GetAs%20BP%20Dino%20Rider))
  (Variables|Default|SetDelta%20Seconds DeltaSeconds)
  (Pawn|Input|AddMovementInput _as_bp_dino_rider (Transformation|GetActorForwardVector _as_bp_dino_rider) 1.0 true))

(event EventBeginPlay
  (bind _asbp_dino_rider (Utilities|Casting|CastToBP_DinoRider (Game|GetPlayerCharacter 0)))
  (Variables|Default|SetAs%20BP%20Dino%20Rider _asbp_dino_rider)
  (Transformation|SetRelativeRotation (Variables|/Game/PlayerBPs/Blueprints/BP_DinoRider.BP_DinoRider_C|GetBulletTracer (Variables|Default|GetAs%20BP%20Dino%20Rider)) (Math|Rotator|FindLookatRotation (Transformation|GetWorldLocation (Variables|/Game/PlayerBPs/Blueprints/BP_DinoRider.BP_DinoRider_C|GetCamera (Variables|Default|GetAs%20BP%20Dino%20Rider))) (+ (Transformation|GetWorldLocation (Variables|/Game/PlayerBPs/Blueprints/BP_DinoRider.BP_DinoRider_C|GetCamera (Variables|Default|GetAs%20BP%20Dino%20Rider))) (* (Math|Vector|GetForwardVector (Variables|/Game/PlayerBPs/Blueprints/BP_DinoRider.BP_DinoRider_C|GetCamera (Variables|Default|GetAs%20BP%20Dino%20Rider))) 2e+04))) false false))