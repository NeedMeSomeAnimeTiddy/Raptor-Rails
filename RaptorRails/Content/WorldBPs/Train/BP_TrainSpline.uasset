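; Train actor that drives five car components along its spline at a set speed.
; Tick advances a shared distance and places each car at a fixed offset ahead of it, matching the spline's local location and rotation while applying Car1's scale to all cars.
; When Looping is on, the base distance resets to zero after exceeding the spline length; the offset car positions are not wrapped individually.
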(event EventTick
  (params (DeltaSeconds :type Float%20%28single-precision%29))
  (Variables|Default|SetDistance (+ (* DeltaSeconds (Variables|Default|GetSpeed)) (Variables|Default|GetDistance)))
  (Transformation|SetRelativeTransform (Variables|Default|GetCar1) (Math|Transform|MakeTransform (.location (Spline|GetTransformatDistanceAlongSpline (Variables|Default|GetSpline) (+ (Variables|Default|GetDistance) 1e+04) "Local" false)) (.rotation (Spline|GetTransformatDistanceAlongSpline (Variables|Default|GetSpline) (+ (Variables|Default|GetDistance) 1e+04) "Local" false)) (Variables|/Script/Engine.SceneComponent|GetRelativeScale3D (Variables|Default|GetCar1))) false false)
  (Transformation|SetRelativeTransform (Variables|Default|GetCar2) (Math|Transform|MakeTransform (.location (Spline|GetTransformatDistanceAlongSpline (Variables|Default|GetSpline) (+ (Variables|Default|GetDistance) 11915.0) "Local" false)) (.rotation (Spline|GetTransformatDistanceAlongSpline (Variables|Default|GetSpline) (+ (Variables|Default|GetDistance) 11915.0) "Local" false)) (Variables|/Script/Engine.SceneComponent|GetRelativeScale3D (Variables|Default|GetCar1))) false false)
  (Transformation|SetRelativeTransform (Variables|Default|GetCar3) (Math|Transform|MakeTransform (.location (Spline|GetTransformatDistanceAlongSpline (Variables|Default|GetSpline) (+ (Variables|Default|GetDistance) 1.383e+04) "Local" false)) (.rotation (Spline|GetTransformatDistanceAlongSpline (Variables|Default|GetSpline) (+ (Variables|Default|GetDistance) 1.383e+04) "Local" false)) (Variables|/Script/Engine.SceneComponent|GetRelativeScale3D (Variables|Default|GetCar1))) false false)
  (Transformation|SetRelativeTransform (Variables|Default|GetCar4) (Math|Transform|MakeTransform (.location (Spline|GetTransformatDistanceAlongSpline (Variables|Default|GetSpline) (+ (Variables|Default|GetDistance) 15745.0) "Local" false)) (.rotation (Spline|GetTransformatDistanceAlongSpline (Variables|Default|GetSpline) (+ (Variables|Default|GetDistance) 15745.0) "Local" false)) (Variables|/Script/Engine.SceneComponent|GetRelativeScale3D (Variables|Default|GetCar1))) false false)
  (Transformation|SetRelativeTransform (Variables|Default|GetCar5) (Math|Transform|MakeTransform (.location (Spline|GetTransformatDistanceAlongSpline (Variables|Default|GetSpline) (+ (Variables|Default|GetDistance) 1.72e+04) "Local" false)) (.rotation (Spline|GetTransformatDistanceAlongSpline (Variables|Default|GetSpline) (+ (Variables|Default|GetDistance) 1.72e+04) "Local" false)) (Variables|/Script/Engine.SceneComponent|GetRelativeScale3D (Variables|Default|GetCar1))) false false)
  (if (Variables|Default|GetLooping?)
    (if (> (Variables|Default|GetDistance) (Spline|GetSplineLength (Variables|Default|GetSpline)))
      (Variables|Default|SetDistance 0.0))))

(fn ConstructionScript)