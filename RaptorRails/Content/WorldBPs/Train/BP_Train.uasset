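; Train actor that moves five car components along the spline of the BP_TrainSpline actor it finds on BeginPlay.
; Five timelines, one per car, play at a rate of 1/SplineTime and set each car's world location and rotation from the spline.
; Each car lerps from its own staggered start distance to the shared spline end, so gaps shrink as the timeline alpha approaches 1.
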(event Custom|TrainAlongSpline
  (bind _trainsplineref (Variables|Default|GetTrainSplineREF))
  (bind _trainsplineref_2 (Variables|Default|GetTrainSplineREF))
  (bind _trainsplineref_3 (Variables|Default|GetTrainSplineREF))
  (bind _trainsplineref_4 (Variables|Default|GetTrainSplineREF))
  (bind _trainsplineref_5 (Variables|Default|GetTrainSplineREF))
  (bind _spline (Variables|/Game/WorldBPs/Train/BP_TrainSpline.BP_TrainSpline_C|GetSpline _trainsplineref))
  (bind _spline_2 (Variables|/Game/WorldBPs/Train/BP_TrainSpline.BP_TrainSpline_C|GetSpline _trainsplineref_2))
  (bind _spline_3 (Variables|/Game/WorldBPs/Train/BP_TrainSpline.BP_TrainSpline_C|GetSpline _trainsplineref_3))
  (bind _spline_4 (Variables|/Game/WorldBPs/Train/BP_TrainSpline.BP_TrainSpline_C|GetSpline _trainsplineref_4))
  (bind _spline_5 (Variables|/Game/WorldBPs/Train/BP_TrainSpline.BP_TrainSpline_C|GetSpline _trainsplineref_5))
  (Components|Timeline|SetPlayRate (Variables|Default|GetAlongSplineTL) (/ 1.0 (Variables|Default|GetSplineTime)))
  (Utilities|FlowControl|Sequence
    (:then_0
      (bind _newtrack_0 (Timeline|AlongSplineTL Play)
        (:Update
          (Transformation|SetWorldTransform (Variables|Default|GetBP_TrainCar4) (Math|Transform|MakeTransform (Math|Vector|MakeVector (.x (Spline|GetLocationatDistanceAlongSpline _spline_2 (Math|Float|Lerp 1.6e+04 (Spline|GetSplineLength (Variables|/Game/WorldBPs/Train/BP_TrainSpline.BP_TrainSpline_C|GetSpline (Variables|Default|GetTrainSplineREF))) _newtrack_0) "World")) (.y (Spline|GetLocationatDistanceAlongSpline _spline_2 (Math|Float|Lerp 1.6e+04 (Spline|GetSplineLength (Variables|/Game/WorldBPs/Train/BP_TrainSpline.BP_TrainSpline_C|GetSpline (Variables|Default|GetTrainSplineREF))) _newtrack_0) "World")) (.z (Spline|GetLocationatDistanceAlongSpline _spline_2 (Math|Float|Lerp 1.6e+04 (Spline|GetSplineLength (Variables|/Game/WorldBPs/Train/BP_TrainSpline.BP_TrainSpline_C|GetSpline (Variables|Default|GetTrainSplineREF))) _newtrack_0) "World"))) (Spline|GetRotationatDistanceAlongSpline _spline_2 (Math|Float|Lerp 1.6e+04 (Spline|GetSplineLength (Variables|/Game/WorldBPs/Train/BP_TrainSpline.BP_TrainSpline_C|GetSpline (Variables|Default|GetTrainSplineREF))) _newtrack_0) "World") "1.000000,1.000000,1.000000") false false))))
    (:then_1
      (bind _newtrack_0_2 (Timeline|AlongSplineTL2 Play)
        (:Update
          (Transformation|SetWorldTransform (Variables|Default|GetBP_TrainCar3) (Math|Transform|MakeTransform (Math|Vector|MakeVector (.x (Spline|GetLocationatDistanceAlongSpline _spline_3 (Math|Float|Lerp 1.275e+04 (Spline|GetSplineLength (Variables|/Game/WorldBPs/Train/BP_TrainSpline.BP_TrainSpline_C|GetSpline (Variables|Default|GetTrainSplineREF))) _newtrack_0_2) "World")) (.y (Spline|GetLocationatDistanceAlongSpline _spline_3 (Math|Float|Lerp 1.275e+04 (Spline|GetSplineLength (Variables|/Game/WorldBPs/Train/BP_TrainSpline.BP_TrainSpline_C|GetSpline (Variables|Default|GetTrainSplineREF))) _newtrack_0_2) "World")) (.z (Spline|GetLocationatDistanceAlongSpline _spline_3 (Math|Float|Lerp 1.275e+04 (Spline|GetSplineLength (Variables|/Game/WorldBPs/Train/BP_TrainSpline.BP_TrainSpline_C|GetSpline (Variables|Default|GetTrainSplineREF))) _newtrack_0_2) "World"))) (Spline|GetRotationatDistanceAlongSpline _spline_3 (Math|Float|Lerp 1.275e+04 (Spline|GetSplineLength (Variables|/Game/WorldBPs/Train/BP_TrainSpline.BP_TrainSpline_C|GetSpline (Variables|Default|GetTrainSplineREF))) _newtrack_0_2) "World") "1.000000,1.000000,1.000000") false false))))
    (:then_2
      (bind _newtrack_0_3 (Timeline|AlongSplineTL3 Play)
        (:Update
          (Transformation|SetWorldTransform (Variables|Default|GetBP_TrainCar2) (Math|Transform|MakeTransform (Math|Vector|MakeVector (.x (Spline|GetLocationatDistanceAlongSpline _spline_4 (Math|Float|Lerp 9.5e+03 (Spline|GetSplineLength (Variables|/Game/WorldBPs/Train/BP_TrainSpline.BP_TrainSpline_C|GetSpline (Variables|Default|GetTrainSplineREF))) _newtrack_0_3) "World")) (.y (Spline|GetLocationatDistanceAlongSpline _spline_4 (Math|Float|Lerp 9.5e+03 (Spline|GetSplineLength (Variables|/Game/WorldBPs/Train/BP_TrainSpline.BP_TrainSpline_C|GetSpline (Variables|Default|GetTrainSplineREF))) _newtrack_0_3) "World")) (.z (Spline|GetLocationatDistanceAlongSpline _spline_4 (Math|Float|Lerp 9.5e+03 (Spline|GetSplineLength (Variables|/Game/WorldBPs/Train/BP_TrainSpline.BP_TrainSpline_C|GetSpline (Variables|Default|GetTrainSplineREF))) _newtrack_0_3) "World"))) (Spline|GetRotationatDistanceAlongSpline _spline_4 (Math|Float|Lerp 9.5e+03 (Spline|GetSplineLength (Variables|/Game/WorldBPs/Train/BP_TrainSpline.BP_TrainSpline_C|GetSpline (Variables|Default|GetTrainSplineREF))) _newtrack_0_3) "World") "1.000000,1.000000,1.000000") false false))))
    (:then_3
      (bind _newtrack_0_4 (Timeline|AlongSplineTL4 Play)
        (:Update
          (Transformation|SetWorldTransform (Variables|Default|GetBP_TrainCar1) (Math|Transform|MakeTransform (Math|Vector|MakeVector (.x (Spline|GetLocationatDistanceAlongSpline _spline_5 (Math|Float|Lerp 6.25e+03 (Spline|GetSplineLength (Variables|/Game/WorldBPs/Train/BP_TrainSpline.BP_TrainSpline_C|GetSpline (Variables|Default|GetTrainSplineREF))) _newtrack_0_4) "World")) (.y (Spline|GetLocationatDistanceAlongSpline _spline_5 (Math|Float|Lerp 6.25e+03 (Spline|GetSplineLength (Variables|/Game/WorldBPs/Train/BP_TrainSpline.BP_TrainSpline_C|GetSpline (Variables|Default|GetTrainSplineREF))) _newtrack_0_4) "World")) (.z (Spline|GetLocationatDistanceAlongSpline _spline_5 (Math|Float|Lerp 6.25e+03 (Spline|GetSplineLength (Variables|/Game/WorldBPs/Train/BP_TrainSpline.BP_TrainSpline_C|GetSpline (Variables|Default|GetTrainSplineREF))) _newtrack_0_4) "World"))) (Spline|GetRotationatDistanceAlongSpline _spline_5 (Math|Float|Lerp 6.25e+03 (Spline|GetSplineLength (Variables|/Game/WorldBPs/Train/BP_TrainSpline.BP_TrainSpline_C|GetSpline (Variables|Default|GetTrainSplineREF))) _newtrack_0_4) "World") "1.000000,1.000000,1.000000") false false))))
    (:then_4
      (bind _newtrack_0_5 (Timeline|AlongSplineTL5 Play)
        (:Update
          (Transformation|SetWorldTransform (Variables|Default|GetBP_TrainCar) (Math|Transform|MakeTransform (Math|Vector|MakeVector (.x (Spline|GetLocationatDistanceAlongSpline _spline (Math|Float|Lerp 3e+03 (Spline|GetSplineLength (Variables|/Game/WorldBPs/Train/BP_TrainSpline.BP_TrainSpline_C|GetSpline (Variables|Default|GetTrainSplineREF))) _newtrack_0_5) "World")) (.y (Spline|GetLocationatDistanceAlongSpline _spline (Math|Float|Lerp 3e+03 (Spline|GetSplineLength (Variables|/Game/WorldBPs/Train/BP_TrainSpline.BP_TrainSpline_C|GetSpline (Variables|Default|GetTrainSplineREF))) _newtrack_0_5) "World")) (.z (Spline|GetLocationatDistanceAlongSpline _spline (Math|Float|Lerp 3e+03 (Spline|GetSplineLength (Variables|/Game/WorldBPs/Train/BP_TrainSpline.BP_TrainSpline_C|GetSpline (Variables|Default|GetTrainSplineREF))) _newtrack_0_5) "World"))) (Spline|GetRotationatDistanceAlongSpline _spline (Math|Float|Lerp 3e+03 (Spline|GetSplineLength (Variables|/Game/WorldBPs/Train/BP_TrainSpline.BP_TrainSpline_C|GetSpline (Variables|Default|GetTrainSplineREF))) _newtrack_0_5) "World") "1.000000,1.000000,1.000000") false false))))))

(event EventBeginPlay
  (bind _returnvalue (Actor|GetActorOfClass "/Game/WorldBPs/Train/BP_TrainSpline.BP_TrainSpline_C"))
  (Variables|Default|SetTrainSplineREF _returnvalue)
  (CallFunction|TrainAlongSpline))

(fn ConstructionScript)