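; BP_TrainOLD is a train actor, apparently an older version, whose five car components follow car positions defined by a BP_TrainSpline actor in the level.
; On BeginPlay it finds and caches the first BP_TrainSpline.
; Every Tick it snaps each car to the world location and rotation of the matching Car1–Car5 on that spline actor, doing no movement math of its own.
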(event EventBeginPlay
  (bind _returnvalue (Actor|GetActorOfClass "/Game/WorldBPs/Train/BP_TrainSpline.BP_TrainSpline_C"))
  (Variables|Default|SetTrainSplineREF _returnvalue))

(event EventTick
  (params (DeltaSeconds :type Float%20%28single-precision%29))
  (bind _trainsplineref (Variables|Default|GetTrainSplineREF))
  (bind _trainsplineref_2 (Variables|Default|GetTrainSplineREF))
  (bind _trainsplineref_3 (Variables|Default|GetTrainSplineREF))
  (bind _trainsplineref_4 (Variables|Default|GetTrainSplineREF))
  (bind _trainsplineref_5 (Variables|Default|GetTrainSplineREF))
  (bind _car2 (Variables|/Game/WorldBPs/Train/BP_TrainSpline.BP_TrainSpline_C|GetCar2 _trainsplineref_5))
  (bind _car3 (Variables|/Game/WorldBPs/Train/BP_TrainSpline.BP_TrainSpline_C|GetCar3 _trainsplineref_2))
  (bind _car5 (Variables|/Game/WorldBPs/Train/BP_TrainSpline.BP_TrainSpline_C|GetCar5 _trainsplineref))
  (bind _car4 (Variables|/Game/WorldBPs/Train/BP_TrainSpline.BP_TrainSpline_C|GetCar4 _trainsplineref_3))
  (bind _car1 (Variables|/Game/WorldBPs/Train/BP_TrainSpline.BP_TrainSpline_C|GetCar1 _trainsplineref_4))
  (bind _returnvalue (Transformation|GetWorldTransform _car5))
  (bind _returnvalue_2 (Transformation|GetWorldTransform _car1))
  (bind _returnvalue_3 (Transformation|GetWorldTransform _car2))
  (bind _returnvalue_4 (Transformation|GetWorldTransform _car3))
  (bind _returnvalue_5 (Transformation|GetWorldTransform _car4))
  (Utilities|FlowControl|Sequence
    (:then_0
      (Transformation|SetWorldTransform (Variables|Default|GetBP_TrainCar) (Math|Transform|MakeTransform (.location _returnvalue_2) (.rotation _returnvalue_2) "1.000000,1.000000,1.000000") false false))
    (:then_1
      (Transformation|SetWorldTransform (Variables|Default|GetBP_TrainCar1) (Math|Transform|MakeTransform (.location _returnvalue_3) (.rotation _returnvalue_3) "1.000000,1.000000,1.000000") false false))
    (:then_2
      (Transformation|SetWorldTransform (Variables|Default|GetBP_TrainCar2) (Math|Transform|MakeTransform (.location _returnvalue_4) (.rotation _returnvalue_4) "1.000000,1.000000,1.000000") false false))
    (:then_3
      (Transformation|SetWorldTransform (Variables|Default|GetBP_TrainCar3) (Math|Transform|MakeTransform (.location _returnvalue_5) (.rotation _returnvalue_5) "1.000000,1.000000,1.000000") false false))
    (:then_4
      (Transformation|SetWorldTransform (Variables|Default|GetBP_TrainCar4) (Math|Transform|MakeTransform (.location _returnvalue) (.rotation _returnvalue) "1.000000,1.000000,1.000000") false false))))

(fn ConstructionScript)