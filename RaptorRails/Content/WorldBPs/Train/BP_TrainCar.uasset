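; BP_TrainCar is a train car that populates itself with enemies for the player's dino rider.
; On BeginPlay it caches the player's BP_DinoRider and sets a three-second, non-looping timer to call SpawnEnemies.
; If the rider's CurrentCar is 0 at that point, SpawnEnemies sets five child actor components to BP_Enemy and clears the timer.
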(event EventBeginPlay
  (bind _asbp_dino_rider (Utilities|Casting|CastToBP_DinoRider (Game|GetPlayerCharacter 0)))
  (Variables|Default|SetAs%20BP%20Dino%20Rider _asbp_dino_rider)
  (Utilities|Time|SetTimerbyFunctionName 0 "SpawnEnemies" 3.0))

(fn ConstructionScript)

(fn SpawnEnemies
  (if (== (Variables|/Game/PlayerBPs/Blueprints/BP_DinoRider.BP_DinoRider_C|GetCurrentCar (Variables|Default|GetAs%20BP%20Dino%20Rider)) 0)
    (ChildActorComponent|SetChildActorClass (Variables|Default|GetChildActor4) "/Game/WorldBPs/Enemy/BP_Enemy.BP_Enemy_C")
    (Utilities|Time|ClearTimerbyFunctionName 0 "SpawnEnemies")))