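; BP_TrainCar1 is a train car with five cube enemies that gates the BP_DinoRider player's progress.
; A looping timer unhides the cubes once the player's CurrentCar is 1.
; Shot toggles a cube's visibility and disables its collision.
; A second timer polls until all five are invisible, then lowers the rider's clamped SplineTime by NextCar, increments CurrentCar and stops.
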(event Custom|IsClear?
  (bind _as_bp_dino_rider (Variables|Default|GetAs%20BP%20Dino%20Rider))
  (if (Math|Boolean|ANDBoolean (not (Variables|/Script/Engine.SceneComponent|GetbVisible (Variables|Default|GetCube1))) (not (Variables|/Script/Engine.SceneComponent|GetbVisible (Variables|Default|GetCube2))) (not (Variables|/Script/Engine.SceneComponent|GetbVisible (Variables|Default|GetCube3))) (not (Variables|/Script/Engine.SceneComponent|GetbVisible (Variables|Default|GetCube4))) (not (Variables|/Script/Engine.SceneComponent|GetbVisible (Variables|Default|GetCube5))))
    (Variables|/Game/PlayerBPs/Blueprints/BP_DinoRider.BP_DinoRider_C|SetSplineTime _as_bp_dino_rider (Math|Float|Clamp(Float) (- (Variables|/Game/PlayerBPs/Blueprints/BP_DinoRider.BP_DinoRider_C|GetSplineTime _as_bp_dino_rider) (Variables|Default|GetNextCar)) 3e+01 6e+01))
    (Variables|/Game/PlayerBPs/Blueprints/BP_DinoRider.BP_DinoRider_C|SetCurrentCar _as_bp_dino_rider (+ (Variables|/Game/PlayerBPs/Blueprints/BP_DinoRider.BP_DinoRider_C|GetCurrentCar _as_bp_dino_rider) 1))
    (Utilities|Time|ClearandInvalidateTimerbyHandle (stale EventBeginPlay _returnvalue))))

(event EventBeginPlay
  (bind _returnvalue (Utilities|Time|SetTimerbyEvent (delegate Custom|IsClear?) 1.0 true))
  (bind _asbp_dino_rider (Utilities|Casting|CastToBP_DinoRider (Game|GetPlayerCharacter 0)))
  (Variables|Default|SetAs%20BP%20Dino%20Rider _asbp_dino_rider)
  (Utilities|Time|SetTimerbyFunctionName 0 "SpawnEnemies" 3.0 true))

(event EventShot
  (params (Enemy :type Primitive%20Component%20Object%20Reference))
  (Rendering|ToggleVisibility Enemy false)
  (Collision|SetCollisionEnabled Enemy "NoCollision"))

(fn ConstructionScript)

(fn SpawnEnemies
  (if (== (Variables|/Game/PlayerBPs/Blueprints/BP_DinoRider.BP_DinoRider_C|GetCurrentCar (Variables|Default|GetAs%20BP%20Dino%20Rider)) 1)
    (Development|SetHiddeninGame (Variables|Default|GetCube3) false false)
    (Utilities|Time|ClearTimerbyFunctionName 0 "SpawnEnemies")))