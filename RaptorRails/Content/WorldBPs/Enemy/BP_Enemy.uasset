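; BP_Enemy is a shootable enemy that tracks health and death and credits kills to the player's BP_DinoRider, cached on BeginPlay.
; Shot passes the hit bone to BodyPartsWIP, which deals heavy damage for Head or Neck and less elsewhere.
; A lethal hit sets Dead, unpossesses the AI controller and increments EnemiesKilled.
; Shots at zero health also reach an increment, behind a separate DoOnce.
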(event EventShot
  (params (Bone :type Name :default "None"))
  (CallFunction|BodyPartsWIP Bone))

(event EventBeginPlay
  (bind _asbp_dino_rider (Utilities|Casting|CastToBP_DinoRider (Game|GetPlayerCharacter 0)))
  (Variables|Default|SetAs%20BP%20Dino%20Rider _asbp_dino_rider))

(fn ConstructionScript)

(fn BodyPartsWIP
  (params (Bone :type Name))
  (bind _as_bp_dino_rider (Variables|Default|GetAs%20BP%20Dino%20Rider))
  (bind _as_bp_dino_rider_2 (Variables|Default|GetAs%20BP%20Dino%20Rider))
  (if (<= (Variables|Default|GetHealth) 0.0)
    (Variables|Default|SetDead? true)
    (Utilities|FlowControl|DoOnce false
      (:Completed
        (Variables|/Game/PlayerBPs/Blueprints/BP_DinoRider.BP_DinoRider_C|SetEnemiesKilled _as_bp_dino_rider (+ (Variables|/Game/PlayerBPs/Blueprints/BP_DinoRider.BP_DinoRider_C|GetEnemiesKilled _as_bp_dino_rider) 1))))
    (else
      (if (or (== Bone "Head") (== Bone "Neck"))
        (Variables|Default|SetHealth (- (Variables|Default|GetHealth) 1e+02))
        (else
          (Variables|Default|SetHealth (- (Variables|Default|GetHealth) 25.0))))
      (if (<= (Variables|Default|GetHealth) 0.0)
        (Variables|Default|SetDead? true)
        (Pawn|UnPossess (AI|GetAIController self))
        (Utilities|FlowControl|DoOnce false
          (:Completed
            (Variables|/Game/PlayerBPs/Blueprints/BP_DinoRider.BP_DinoRider_C|SetEnemiesKilled _as_bp_dino_rider_2 (+ (Variables|/Game/PlayerBPs/Blueprints/BP_DinoRider.BP_DinoRider_C|GetEnemiesKilled _as_bp_dino_rider_2) 1))))))))

(fn CheckMatchingGameplayTag
  (params (Tag%20Container :type Gameplay%20Tag%20Container%20Structure))
  (return false))