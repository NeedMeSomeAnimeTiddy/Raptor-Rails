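; BP_Pillar is an obstacle that turns physical when the player nears it and punishes the rider on impact.
; A one-time overlap on its box enables physics simulation on the cube.
; Cube hits pass a DoOnce to cut the BP_DinoRider's walk speed, apply damage, tag the player controller as slowed and regulate speed.
; A short timer removes the tag and re-arms the hit.
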(event OnComponentBeginOverlap(B0x)
  (params (OverlappedComponent :type Primitive%20Component%20Object%20Reference) (OtherActor :type Actor%20Object%20Reference) (OtherComp :type Primitive%20Component%20Object%20Reference) (OtherBodyIndex :type Integer) (bFromSweep :type Boolean) (SweepResult :type Hit%20Result%20Structure%20%28by%20ref%29))
  (if (== OtherActor (Game|GetPlayerCharacter 0))
    (Utilities|FlowControl|DoOnce false
      (:Completed
        (Physics|SetSimulatePhysics (Variables|Default|GetCube) true)))))

(event OnComponentHit(Cube)
  (params (HitComponent :type Primitive%20Component%20Object%20Reference) (OtherActor :type Actor%20Object%20Reference) (OtherComp :type Primitive%20Component%20Object%20Reference) (NormalImpulse :type Vector :default "0, 0, 0") (Hit :type Hit%20Result%20Structure%20%28by%20ref%29))
  (bind _asbp_dino_rider (Utilities|Casting|CastToBP_DinoRider OtherActor))
  (if (== OtherActor (Game|GetPlayerCharacter 0))
    (Utilities|FlowControl|DoOnce false
      (:Completed
        (Variables|/Script/Engine.CharacterMovementComponent|SetMaxWalkSpeed (Variables|/Script/Engine.Character|GetCharacterMovement _asbp_dino_rider) (Math|Float|Clamp(Float) (- (Variables|/Script/Engine.CharacterMovementComponent|GetMaxWalkSpeed (Variables|/Script/Engine.Character|GetCharacterMovement _asbp_dino_rider)) 1.3e+03) 0.0 1.3e+03))
        (Game|Damage|ApplyDamage _asbp_dino_rider 5e+01 0 0)
        (bind _asbp_player_controller (Utilities|Casting|CastToBP_PlayerController (Game|GetPlayerController 0)))
        (GameplayTags|AddGameplayTag (Variables|/Game/PlayerBPs/Blueprints/BP_PlayerController.BP_PlayerController_C|GetGameplayTags _asbp_player_controller) "(TagName=\"Player.State.Slowed\")" :!class /Script/GameplayTags.BlueprintGameplayTagLibrary)
        (Default|RegulateSpeed _asbp_player_controller)
        (Utilities|Time|SetTimerbyEvent (delegate Custom|ResetSlowed) 1.0)))))

(event Custom|ResetSlowed
  (GameplayTags|RemoveGameplayTag (Variables|/Game/PlayerBPs/Blueprints/BP_PlayerController.BP_PlayerController_C|GetGameplayTags (stale OnComponentHit(Cube) _asbp_player_controller)) "(TagName=\"Player.State.Slowed\")" :!class /Script/GameplayTags.BlueprintGameplayTagLibrary)
  (CallFunction|ResetSlowdown))

(event Custom|ResetSlowdown
  (Utilities|FlowControl|DoOnce false) ; enters at Reset
)

(fn ConstructionScript)

(fn CheckMatchingGameplayTag
  (params (Tag%20Container :type Gameplay%20Tag%20Container%20Structure))
  (return (GameplayTags|MatchesAnyTags (Variables|Default|GetGameplayTag) Tag%20Container)))